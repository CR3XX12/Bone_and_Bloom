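; BP_KnightPrisoner is a knight prisoner character that loops an idle animation from BeginPlay.
; Its Interact event casts the instigator's PlayerState to CS_PlayerState, awards EarnedXp, then calls CharacterCheer to switch to a looping cheer animation.
; Animations play directly on the skeletal mesh.
; CanInteract always returns false, and Interact itself has no guard against repeated XP awards.
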(event Custom|CharacterCheer
  (Components|Animation|PlayAnimation (Variables|Default|GetSkeletalMesh) (Variables|Default|GetMontageCheer) true))

(event EventBeginPlay
  (Components|Animation|PlayAnimation (Variables|Default|GetSkeletalMesh) (Variables|Default|GetMontageIdle) true))

(event EventInteract
  (params (CharacterInstigator :type CS%20Character%20Object%20Reference))
  (bind _ascs_player_state (Utilities|Casting|CastToCS_PlayerState (Variables|/Script/Engine.Pawn|GetPlayerState CharacterInstigator)))
  (Class|CSPlayerState|AddXp _ascs_player_state (Variables|Default|GetEarnedXp))
  (CallFunction|CharacterCheer))

(fn ConstructionScript)

(fn CanInteract
  (params (CharacterInstigator :type CS%20Character%20Object%20Reference))
  (return false))